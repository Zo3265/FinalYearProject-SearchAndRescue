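; Manager actor for Learning Agents enemies that trains or runs their neural network policy.
; BeginPlay makes the enemies tick after it, builds the interactor, policy, critic and training environment, and passes the level spline to interactor and environment.
; It also spawns a shared-memory trainer process feeding a PPO trainer.
; RunInference switches Tick between training and inference, and in inference mode scatters enemies to random spline points at start.
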(event `self.ReceiveBeginPlay`
  (bind _shared_memory_settings (`self.Shared Memory Settings`))
  (`KismetSystemLibrary.PrintString` "Started")
  (`|ExecutionSequence`
    (:`then_0`
      (bind _outactors (`GameplayStatics.GetAllActorsOfClass` "/Game/MLAI/MLEnemyBase/BP_MLEnemyBase.BP_MLEnemyBase_C"))
      (bind _output_get (set `self.EnemyActorArray` _outactors))
      (`self.AddTickPrerequisiteActor` _output_get self))
    (:`then_1`
      (bind _returnvalue (`GameplayStatics.GetActorOfClass` "/Game/AI/EnemyBase/BP_SplineController.BP_SplineController_C"))
      (set `self.BPManagerSpline` (`SplineController.Spline` _returnvalue)))
    (:`then_2`
      (bind _returnvalue_2 (`LearningAgentsInteractor.MakeInteractor` (`self.LearningAgentsManager`) "/Script/SearchAndRescue.EnemyInteractor" "EnemyInteractor"))
      (bind _output_get_2 (set `self.Interactor` _returnvalue_2))
      (`EnemyInteractor.setInteractorSplineComponent` _output_get_2 (`self.BPManagerSpline`)))
    (:`then_3`
      (bind _returnvalue_3 (`LearningAgentsPolicy.MakePolicy` (`self.LearningAgentsManager`) (`self.Interactor`) "/Script/LearningAgents.LearningAgentsPolicy" "EnemyPolicy" "/Game/MLAI/NeuralNetwrokAssets/DA_Encoder.DA_Encoder" "/Game/MLAI/NeuralNetwrokAssets/DA_Policy.DA_Policy" "/Game/MLAI/NeuralNetwrokAssets/DA_Decoder.DA_Decoder" true true true (`self.Policy Settings`)))
      (set `self.Policy` _returnvalue_3))
    (:`then_4`
      (bind _returnvalue_4 (`LearningAgentsCritic.MakeCritic` (`self.LearningAgentsManager`) (`self.Interactor`) (`self.Policy`) "/Script/LearningAgents.LearningAgentsCritic" "EnemyCritic" "/Game/MLAI/NeuralNetwrokAssets/DA_Critic.DA_Critic" true (`self.Critic Settings`)))
      (set `self.Critic` _returnvalue_4))
    (:`then_5`
      (bind _returnvalue_5 (`LearningAgentsTrainingEnvironment.MakeTrainingEnvironment` (`self.LearningAgentsManager`) "/Script/SearchAndRescue.EnemyTrainingEnvironment" "EnemyTrainingEnvironment"))
      (bind _output_get_3 (set `self.TrainingEnv` _returnvalue_5))
      (`EnemyTrainingEnvironment.setTrainingEnvSplineComponent` _output_get_3 (`self.BPManagerSpline`)))
    (:`then_6`
      (bind _returnvalue_6 (`LearningAgentsCommunicatorLibrary.SpawnSharedMemoryTrainingProcess` (`self.Trainer Process Settings`) _shared_memory_settings))
      (bind _returnvalue_7 (`LearningAgentsCommunicatorLibrary.MakeSharedMemoryCommunicator` _returnvalue_6 _shared_memory_settings))
      (set `self.Communicator` _returnvalue_7))
    (:`then_7`
      (bind _returnvalue_8 (`LearningAgentsPPOTrainer.MakePPOTrainer` (`self.LearningAgentsManager`) (`self.Interactor`) (`self.TrainingEnv`) (`self.Policy`) (`self.Critic`) (`self.Communicator`) "/Script/LearningAgentsTraining.LearningAgentsPPOTrainer" "PPOTrainer" (`self.Trainer Settings`)))
      (set `self.ManagerPPOTrainer` _returnvalue_8))
    (:`then_8`
      (if (`self.RunInference`)
        (`MLEnemyBase.ResetToRandomPointOnSpline` (`self.EnemyActorArray`))))))

(event `self.ReceiveTick`
  (params (DeltaSeconds :type "Float (single-precision)"))
  (if (`self.RunInference`)
    (`LearningAgentsPolicy.RunInference` (`self.Policy`) 1.0)
    (else
      (`LearningAgentsPPOTrainer.RunTraining` (`self.ManagerPPOTrainer`) (`self.Trainer Training Settings`) (`self.Training Game Settings`) true true))))

(fn `UserConstructionScript`)